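; Roamer AI bot that, based on its state at BeginPlay, either chases the player or patrols between target points with pauses.
; Chase uses AIMoveTo, then on arrival spawns an explosion, calls ApplyDamage and destroys the bot; Roam also maps to Chase.
; Pawn sensing, or the T key, moves it toward a ThirdPersonCharacter, falling back to patrol on failure.
; Its box overlap teleports the overlapping actor to Teleport1.
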(event OnSeePawn(PawnSensing)
  (params (Pawn :type Pawn%20Object%20Reference))
  (Development|PrintString "Hello")
  (bind _asthird_person_character (Utilities|Casting|CastToThirdPersonCharacter Pawn))
  (AI|AIMoveTo self "0, 0, 0" _asthird_person_character 5.0 false
    (:OnFail
      (CallFunction|Patrol))))

(event OnComponentBeginOverlap(Box)
  (params (OverlappedComponent :type Primitive%20Component%20Object%20Reference) (OtherActor :type Actor%20Object%20Reference) (OtherComp :type Primitive%20Component%20Object%20Reference) (OtherBodyIndex :type Integer) (bFromSweep :type Boolean) (SweepResult :type Hit%20Result%20Structure%20%28by%20ref%29))
  (Transformation|Teleport OtherActor (Transformation|GetActorLocation (Variables|Default|Getteleport1)) "0, 0, 0"))

(event Custom|patrol
  (AI|AIMoveTo self "0, 0, 0" self 5.0 false
    (:OnSuccess
      (Utilities|FlowControl|Delay 2.0)
      (AI|AIMoveTo self "0, 0, 0" (Variables|Default|Gettargetpoint3) 5.0 false
        (:OnSuccess
          (Utilities|FlowControl|Delay 2.0)
          (AI|AIMoveTo self "0, 0, 0" (Variables|Default|Gettargetpoint1) 5.0 false
            (:OnSuccess
              _)
            (:OnFail
              _))
          (CallFunction|Patrol))))))

(event Custom|chase
  (bind _returnvalue (Transformation|GetActorLocation))
  (AI|AIMoveTo self "0, 0, 0" (Game|GetPlayerCharacter 0) 5.0 false
    (:OnSuccess
      (Effects|SpawnEmitteratLocation "/Game/StarterContent/Particles/P_Explosion.P_Explosion" _returnvalue)
      (Game|Damage|ApplyDamage 0 5.0 0 0)
      (Audio|PlaySoundatLocation "/Game/StarterContent/Audio/Explosion01.Explosion01" _returnvalue)
      (Actor|DestroyActor))))

(event EventBeginPlay
  (switch Utilities|FlowControl|Switch|Switchoneaistate (Variables|Default|Getaistate)
    (:NewEnumerator1
      (CallFunction|Chase))
    (:NewEnumerator2
      (CallFunction|Chase))
    (:NewEnumerator3
      (CallFunction|Patrol))))

(event Input|KeyboardEvents|T
  (params (Key :type Key%20Structure))
  (:Pressed
    (bind _asthird_person_character (Utilities|Casting|CastToThirdPersonCharacter (stale OnSeePawn(PawnSensing) Pawn)))
    (AI|AIMoveTo self "0, 0, 0" _asthird_person_character 5.0 false
      (:OnFail
        (CallFunction|Patrol)))))

(fn ConstructionScript)