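; Roamer bot pawn meant to patrol through an array of patrol points, starting on BeginPlay.
; PatrolTopoint runs AI MoveTo on itself, then on success advances the index and calls itself again, looping indefinitely while moves succeed.
; The index wraps to 1 rather than 0, and failed moves are unhandled.
; The current patrol point lookup is unconnected, so the move receives no destination from the array.
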(event Custom|patrolTopoint
  (AI|AIMoveTo self "0, 0, 0" 0 5.0 false
    (:OnSuccess
      (if (>= (Variables|Default|Getpatrolpointint) (- (Utilities|Array|Length (Variables|Default|Getpatrolpoints)) 1))
        (Variables|Default|Setpatrolpointint 1)
        (else
          (Math|Integer|IncrementInt (Variables|Default|Getpatrolpointint)
            (:%20%20
              _))))
      (CallFunction|PatrolTopoint))))

(event EventBeginPlay
  (CallFunction|PatrolTopoint))

(fn ConstructionScript)